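; BP_RTActor is a scene capture actor that switches its SceneCaptureComponent2D between showing cube actors and sphere actors.
; On BeginPlay it caches all actors tagged "Cube" and "Sphere" into two arrays.
; The ChangeView event assigns one of these arrays to the capture component's ShowOnlyActors list, selected by the IsCubes flag.
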(event Custom|ChangeView
  (params (IsCubes? :type Boolean))
  (bind _scenecapturecomponent2d (Variables|Default|GetSceneCaptureComponent2D))
  (if IsCubes?
    (Variables|/Script/Engine.SceneCaptureComponent|SetShowOnlyActors _scenecapturecomponent2d (Variables|Default|GetCubes))
    (else
      (Variables|/Script/Engine.SceneCaptureComponent|SetShowOnlyActors _scenecapturecomponent2d (Variables|Default|GetSpheres)))))

(event EventBeginPlay
  (bind _outactors (Actor|GetAllActorsOfClasswithTag "/Script/Engine.Actor" "Cube"))
  (Variables|Default|SetCubes _outactors)
  (bind _outactors_2 (Actor|GetAllActorsOfClasswithTag "/Script/Engine.Actor" "Sphere"))
  (Variables|Default|SetSpheres _outactors_2))

(event Collision|EventActorBeginOverlap
  (params (OtherActor :type Actor%20Object%20Reference)))

(event EventTick
  (params (DeltaSeconds :type Float%20%28single-precision%29)))

(fn ConstructionScript)